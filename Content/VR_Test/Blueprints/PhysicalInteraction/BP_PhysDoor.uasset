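; BP_PhysDoor is a physics-driven door in the VR test content that can start locked.
; An unlocked door enables physics simulation at BeginPlay, while a locked one does so on Interact, which also clears the lock.
; Every Tick, DoorHolder flip-flops the physics constraint's angular velocity target between opposite Y values, apparently to hold the door steady, and is flagged as expensive.
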(event EventBeginPlay
  (if (not (Variables|Default|GetbIsLocked))
    (Physics|SetSimulatePhysics (Variables|Default|GetDoor) true)
    (Variables|Default|SetbIsLocked false)))

(event Collision|EventActorBeginOverlap
  (params (OtherActor :type Actor%20Object%20Reference)))

(event EventTick
  (params (DeltaSeconds :type Float%20%28single-precision%29))
  ;[1 1 1] EXPENSIVE! Change mb?
  (CallFunction|DoorHolder))

(event EventInteract
  (if (Variables|Default|GetbIsLocked)
    (Physics|SetSimulatePhysics (Variables|Default|GetDoor) true)
    (Variables|Default|SetbIsLocked false)))

(fn ConstructionScript)

(fn DoorHolder
  (Utilities|FlowControl|FlipFlop
    (:A
      (Class|PhysicsConstraintComponent|SetAngularVelocityTarget (Variables|Default|GetPhysicsConstraint) (Math|Vector|MakeVector 0.0 1.0 0.0)))
    (:B
      (Class|PhysicsConstraintComponent|SetAngularVelocityTarget (Variables|Default|GetPhysicsConstraint) (Math|Vector|MakeVector 0.0 -1.0 0.0)))))