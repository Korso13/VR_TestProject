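; BP_PhysButton is a physical button for VR interaction that activates an assigned AffectedActor when pushed.
; On BeginPlay it stores a threshold 3 units below the button's starting relative location on each axis.
; Tick checks whether any axis reaches that threshold and sends InteractMessage through BPI_Interaction, if the actor implements it.
; A DoOnce limits this to one message per press and resets once the button is back above the threshold.
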(event EventBeginPlay
  (bind _button (Variables|Default|GetButton))
  (bind _relativelocation (Variables|/Script/Engine.SceneComponent|GetRelativeLocation _button))
  (Variables|Default|SetTrigger%20Vector (Math|Vector|MakeVector (- (.x _relativelocation) 3.0) (- (.y _relativelocation) 3.0) (- (.z _relativelocation) 3.0))))

(event Collision|EventActorBeginOverlap
  (params (OtherActor :type Actor%20Object%20Reference)))

(event EventTick
  (params (DeltaSeconds :type Float%20%28single-precision%29))
  (bind _button (Variables|Default|GetButton))
  (bind _affectedactor (Variables|Default|GetAffectedActor))
  (bind _trigger_vector (Variables|Default|GetTrigger%20Vector))
  (bind _relativelocation (Variables|/Script/Engine.SceneComponent|GetRelativeLocation _button))
  (if (Math|Boolean|ORBoolean (<= (.x _relativelocation) (.x _trigger_vector)) (<= (.y _relativelocation) (.y _trigger_vector)) (<= (.z _relativelocation) (.z _trigger_vector)))
    (Utilities|FlowControl|DoOnce false :!label _label
      (:Completed
        (if (Utilities|DoesObjectImplementInterface _affectedactor "/Game/VR_Test/Blueprints/BPI_Interaction.BPI_Interaction_C")
          (Class|BPIInteraction|Interact(Message) _affectedactor))))
    (else
      (goto _label Reset))))

(fn ConstructionScript)