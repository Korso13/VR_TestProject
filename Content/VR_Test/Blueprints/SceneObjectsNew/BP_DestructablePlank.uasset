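; Destructible plank actor that loses durability when damaged and collapses into debris.
; TakeDurabilityDamage subtracts damage while durability remains and plays a 2D hit sound.
; At zero or below it plays a collapse sound, clears the mesh, disables its collision and spawns half-scale BP_RandomDebris at two spawn points.
; The actor is not destroyed, and its event graph is empty, so damage relies on calls to that function.
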(event EventBeginPlay)

(event Collision|EventActorBeginOverlap
  (params (OtherActor :type Actor%20Object%20Reference)))

(event EventTick
  (params (DeltaSeconds :type Float%20%28single-precision%29)))

(fn ConstructionScript)

(fn TakeDurabilityDamage
  (params (DamageValue :type Integer))
  (bind _debrisspawn2 (Variables|Default|GetDebrisSpawn2))
  (bind _debrisspawn1 (Variables|Default|GetDebrisSpawn1))
  (bind _staticmesh (Variables|Default|GetStaticMesh))
  (bind _returnvalue (Transformation|GetWorldTransform _debrisspawn1))
  (bind _returnvalue_2 (Transformation|GetWorldTransform _debrisspawn2))
  (if (> (Variables|Default|GetDurability) 0)
    (bind _output_get (Variables|Default|SetDurability (- (Variables|Default|GetDurability) DamageValue)))
    (Audio|PlaySound2D "/Engine/VREditor/Sounds/UI/Object_Snaps_To_Grid.Object_Snaps_To_Grid" 1.0 1.0 0.0 0 0)
    (if (<= _output_get 0)
      (Audio|PlaySound2D "/Game/StarterContent/Audio/Collapse01.Collapse01" 0.5 1.5 0.0 0 0)
      (Components|StaticMesh|SetStaticMesh _staticmesh 0)
      (Collision|SetCollisionEnabled _staticmesh "NoCollision")
      (Game|SpawnActorfromClass "/Game/VR_Test/Blueprints/PhysBasedGrabObjects/BP_RandomDebris.BP_RandomDebris_C" (Math|Transform|MakeTransform (.location _returnvalue) (.rotation _returnvalue) "0.500000,0.500000,0.500000") "AlwaysSpawn" self (Game|Player|GetPlayerPawn 0))
      (Game|SpawnActorfromClass "/Game/VR_Test/Blueprints/PhysBasedGrabObjects/BP_RandomDebris.BP_RandomDebris_C" (Math|Transform|MakeTransform (.location _returnvalue_2) (.rotation _returnvalue_2) "0.500000,0.500000,0.500000") "AlwaysSpawn" self (Game|Player|GetPlayerPawn 0)))))