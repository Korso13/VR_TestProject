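; BP_BaseGrabActor is a base VR grabbable actor whose static mesh can be picked up and released by an interacting component.
; Grab turns off physics simulation and attaches the mesh to that component, while Release restores physics and detaches it.
; Attach and detach live in separate overridable functions, keeping world transforms by default, so child Blueprints can customize how objects attach.
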(event EventBeginPlay)

(event Collision|EventActorBeginOverlap
  (params (OtherActor :type Actor%20Object%20Reference)))

(event EventTick
  (params (DeltaSeconds :type Float%20%28single-precision%29)))

(event EventGrab
  (params (Interacting%20Component :type Primitive%20Component%20Object%20Reference))
  (bind _staticmesh (Variables|Default|GetStaticMesh))
  ;[1 1 1] Item Grab mechanic
  (Physics|SetSimulatePhysics _staticmesh false)
  ;;[0.3836 0.2325 1] Can be overriden to customize attachment rules
  (CallFunction|OnGrabAttachActor _staticmesh Interacting%20Component))

(event EventRelease
  (bind _staticmesh (Variables|Default|GetStaticMesh))
  ;[1 1 1] Item Grab mechanic
  (Physics|SetSimulatePhysics _staticmesh true)
  ;;[0.3836 0.2325 1] For customizable detaching
  (CallFunction|OnReleaseDetachActor _staticmesh))

(fn ConstructionScript)

(fn OnGrabAttachActor
  (params (ComponentToAttach :type Primitive%20Component%20Object%20Reference) (TargetComponent :type Primitive%20Component%20Object%20Reference))
  (Transformation|AttachComponentToComponent ComponentToAttach TargetComponent "None" "KeepWorld" "KeepWorld" "KeepWorld" true))

(fn OnReleaseDetachActor
  (params (Detaching%20Component :type Primitive%20Component%20Object%20Reference))
  (Transformation|DetachFromComponent Detaching%20Component "KeepWorld" "KeepWorld" "KeepWorld" true))