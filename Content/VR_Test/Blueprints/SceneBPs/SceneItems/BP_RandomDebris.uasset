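; BP_RandomDebris is a short-lived wooden debris actor that picks its mesh at random when spawned.
; On BeginPlay it sets a random debris mesh and an oak material, then enables query and physics collision blocking all channels.
; The selection only reaches the first two of its three meshes, since the random integer never returns the last index.
; After a fixed delay, the actor destroys itself.
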(event EventBeginPlay
  (bind _objectmesh (Variables|Default|GetObjectMesh))
  (|CallParentFunction)
  (Components|StaticMesh|SetStaticMesh _objectmesh (Utilities|Select :Index (Math|Random|RandomInteger 2) :Option%200 "/Game/VR_Test/Meshes/SM_Debris01.SM_Debris01" :Option%201 "/Game/VR_Test/Meshes/SM_Debris02.SM_Debris02" :Option%202 "/Game/VR_Test/Meshes/SM_Debris03.SM_Debris03"))
  (Rendering|Material|SetMaterial _objectmesh 0 "/Game/StarterContent/Materials/M_Wood_Oak.M_Wood_Oak")
  (Collision|SetCollisionEnabled _objectmesh "QueryAndPhysics")
  (Collision|SetCollisionResponsetoAllChannels _objectmesh "ECR_Block")
  (Utilities|FlowControl|Delay 1e+01)
  (Actor|DestroyActor))

(event Collision|EventActorBeginOverlap
  (params (OtherActor :type Actor%20Object%20Reference))
  (|CallParentFunction OtherActor) ; This node is disabled and will not be called.\nDrag off pins to build functionality.
)

(event EventTick
  (params (DeltaSeconds :type Float%20%28single-precision%29))
  (|CallParentFunction DeltaSeconds) ; This node is disabled and will not be called.\nDrag off pins to build functionality.
)

(fn ConstructionScript
  (|CallParentFunction))