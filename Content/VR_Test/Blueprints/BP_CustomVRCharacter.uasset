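; VR character Blueprint that adds arc-aimed teleport movement on the right controller.
; BeginPlay sets eye-level tracking when an HMD is enabled, and pressing the teleport input starts a looping timer.
; Each timer tick traces a debug-drawn projectile path from the controller and projects hits onto the navmesh to place and validate TeleportSpot.
; Release stops the timer and, if valid, moves the actor there with a height offset and matches VRRoot's rotation.
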(event EventBeginPlay
  (if (Class|HeadMountedDisplayFunctionLibrary|IsHeadMountedDisplayEnabled)
    (Class|HeadMountedDisplayFunctionLibrary|SetTrackingOrigin "Eye")))

(event Collision|EventActorBeginOverlap
  (params (OtherActor :type Actor%20Object%20Reference)))

(event EventTick
  (params (DeltaSeconds :type Float%20%28single-precision%29)))

(event Input|ActionEvents|InputActionTeleportRightController
  (params (Key :type Key%20Structure :default "None"))
  (:Pressed
    (CallFunction|StartTeleport))
  (:Released
    (CallFunction|DeactivateTeleport)))

(fn ConstructionScript)

(fn StartTeleport
  (if (not (Variables|Default|GetbTeleportActive))
    (Variables|Default|SetbTeleportActive true)
    (Rendering|SetVisibility (Variables|Default|GetTeleportSpot) true false)
    (bind _returnvalue (Utilities|Time|SetTimerbyFunctionName 0 "UpdateTraceTeleport" 0.1 true))
    (Variables|Default|SetTeleportTimer _returnvalue)))

(fn UpdateTraceTeleport
  (bind _motioncontrollerright (Variables|Default|GetMotionControllerRight))
  (bind _teleportspot (Variables|Default|GetTeleportSpot))
  (bind _outhit (Class|GameplayStatics|BlueprintPredictProjectilePathbyObjectType (Transformation|GetWorldLocation _motioncontrollerright) (* (Math|Vector|GetForwardVector _motioncontrollerright) (LocalVariables|GetVelocity)) true 5.0 (Utilities|Array|MakeArray "ObjectTypeQuery1") false 0 "ForDuration"))
  (if (.bblockinghit _outhit)
    (Transformation|SetWorldLocation _teleportspot (.ProjectedLocation (AI|Navigation|ProjectPointtoNavigation (Class|NavigationSystemV1|GetNavigationSystem) (.location _outhit) 0 0 "200.000000,200.000000,200.000000")) false false)
    (Rendering|SetVisibility _teleportspot (.ReturnValue (AI|Navigation|ProjectPointtoNavigation (Class|NavigationSystemV1|GetNavigationSystem) (.location _outhit) 0 0 "200.000000,200.000000,200.000000")) false)
    (Variables|Default|SetbCanTeleport (.ReturnValue (AI|Navigation|ProjectPointtoNavigation (Class|NavigationSystemV1|GetNavigationSystem) (.location _outhit) 0 0 "200.000000,200.000000,200.000000")))))

(fn DeactivateTeleport
  (bind _teleportspot (Variables|Default|GetTeleportSpot))
  (if (Utilities|Time|IsValidTimerHandle (Variables|Default|GetTeleportTimer))
    (Utilities|Time|ClearandInvalidateTimerbyHandle (Variables|Default|GetTeleportTimer))
    (Variables|Default|SetTeleportTimer "")
    (Variables|Default|SetbTeleportActive false)
    (Rendering|SetVisibility (Variables|Default|GetTeleportSpot) false false)
    (if (Variables|Default|GetbCanTeleport)
      (Transformation|SetActorLocation (+ (Transformation|GetWorldLocation _teleportspot) (Math|Vector|MakeVector 0.0 0.0 (Variables|Default|GetCharacterHeight))) false false)
      (Transformation|SetWorldRotation (Variables|Default|GetVR%20Root) (Transformation|GetWorldRotation _teleportspot) false false))))