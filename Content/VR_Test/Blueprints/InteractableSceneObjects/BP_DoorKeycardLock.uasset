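; BP_DoorKeycardLock is an interactable keycard reader that unlocks its connected door in the VR test scene.
; When KeycardCollision is overlapped by a BP_Keycard while a valid ConnectedDoor is locked, it waits briefly, then swaps the red light for the green one.
; It then plays a 2D success sound and calls UnlockDoor on that door.
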(event OnComponentBeginOverlap(KeycardCollision)
  (params (OverlappedComponent :type Primitive%20Component%20Object%20Reference) (OtherActor :type Actor%20Object%20Reference) (OtherComp :type Primitive%20Component%20Object%20Reference) (OtherBodyIndex :type Integer) (bFromSweep :type Boolean) (SweepResult :type Hit%20Result%20Structure%20%28by%20ref%29))
  (if (Utilities|IsValid (Variables|Default|GetConnectedDoor))
    (if (Variables|/Game/VR_Test/Blueprints/InteractableSceneObjects/BP_UnlockableDoor.BP_UnlockableDoor_C|GetbIsLocked (Variables|Default|GetConnectedDoor))
      (Utilities|Casting|CastToBP_Keycard OtherActor)
      (Utilities|FlowControl|Delay 0.7)
      (Rendering|SetVisibility (Variables|Default|GetGreenLight) true false)
      (Rendering|SetVisibility (Variables|Default|GetRedLight) false false)
      (Audio|PlaySound2D "/Engine/EditorSounds/Notifications/CompileSuccess.CompileSuccess" 1.0 1.0 0.0 0 0)
      (Default|UnlockDoor (Variables|Default|GetConnectedDoor)))))

(event EventBeginPlay
  (Rendering|SetVisibility (Variables|Default|GetGreenLight) false false))

(event Collision|EventActorBeginOverlap
  (params (OtherActor :type Actor%20Object%20Reference)))

(event EventTick
  (params (DeltaSeconds :type Float%20%28single-precision%29)))

(fn ConstructionScript)