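; BP_BreakableDoor is a door in the VR test content that breaks once its durability runs out.
; TakeDurabilityDamage subtracts damage from DoorDurability and plays a 2D hit sound while the door is intact.
; At zero it plays a collapse sound, clears the mesh and its collision, and spawns BP_RandomDebris actors at randomly selected spawn points.
; The random pick only reaches the first two of the three debris points.
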(event EventBeginPlay)

(event Collision|EventActorBeginOverlap
  (params (OtherActor :type Actor%20Object%20Reference)))

(event EventTick
  (params (DeltaSeconds :type Float%20%28single-precision%29)))

(fn ConstructionScript)

(fn TakeDurabilityDamage
  (params (DamageValue :type Integer))
  (bind _doormesh (Variables|Default|GetDoorMesh))
  (if (> (Variables|Default|GetDoorDurability) 0)
    (bind _output_get (Variables|Default|SetDoorDurability (- (Variables|Default|GetDoorDurability) DamageValue)))
    (Audio|PlaySound2D "/Engine/VREditor/Sounds/UI/Object_Snaps_To_Grid.Object_Snaps_To_Grid" 1.0 1.0 0.0 0 0)
    (if (<= _output_get 0)
      (Audio|PlaySound2D "/Game/StarterContent/Audio/Collapse01.Collapse01" 0.5 1.5 0.0 0 0)
      (Components|StaticMesh|SetStaticMesh _doormesh 0)
      (Collision|SetCollisionEnabled _doormesh "NoCollision")
      (for _index (range 0 4)
        (Game|SpawnActorfromClass "/Game/VR_Test/Blueprints/SceneBPs/SceneItems/BP_RandomDebris.BP_RandomDebris_C" (Transformation|GetWorldTransform (Utilities|Select :Index (Math|Random|RandomInteger 2) :Option%200 (Variables|Default|GetDebrisSpawn1) :Option%201 (Variables|Default|GetDebrisSpawn2) :Option%202 (Variables|Default|GetDebrisSpawn3))) "AlwaysSpawn" self (Game|Player|GetPlayerPawn 0))))))