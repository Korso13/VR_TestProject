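; VR test grabbable box that an interacting component, such as a motion controller, can pick up and drop.
; Grab disables mesh physics and Release re-enables it, with attach and detach delegated to overridable functions.
; Attaching moves GrabSpot to the closest point on the mesh's collision, parents the mesh to it, then attaches GrabSpot to the interacting component.
; Detaching only releases GrabSpot from that component.
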(event EventBeginPlay)

(event Collision|EventActorBeginOverlap
  (params (OtherActor :type Actor%20Object%20Reference)))

(event EventTick
  (params (DeltaSeconds :type Float%20%28single-precision%29)))

(event EventGrab
  (params (Interacting%20Component :type Primitive%20Component%20Object%20Reference))
  (bind _staticmesh1 (Variables|Default|GetStaticMesh1))
  ;[1 1 1] Item Grab mechanic
  (Physics|SetSimulatePhysics _staticmesh1 false)
  ;;[0.3836 0.2325 1] Can be overriden to customize attachment rules
  (CallFunction|OnGrabAttachActor _staticmesh1 Interacting%20Component))

(event EventRelease
  (bind _staticmesh1 (Variables|Default|GetStaticMesh1))
  ;[1 1 1] Item Grab mechanic
  (Physics|SetSimulatePhysics _staticmesh1 true)
  ;;[0.3836 0.2325 1] For customizable detaching
  (CallFunction|OnReleaseDetachActor _staticmesh1))

(fn ConstructionScript
  (|CallParentFunction))

(fn OnGrabAttachActor
  (params (ComponentToAttach :type Primitive%20Component%20Object%20Reference) (TargetComponent :type Primitive%20Component%20Object%20Reference))
  ;[1 1 1] Alternative way
  ;;[0.191 0.2518 1] Moving grab spot to closest point on item's collision
  (Transformation|SetWorldLocation (Variables|Default|GetGrabSpot) (.OutPointOnBody (Collision|GetClosestPointonCollision (Variables|Default|GetStaticMesh1) (Transformation|GetWorldLocation TargetComponent) "None")) false false)
  ;;[0.191 0.2518 1] Forcing the main mesh to follow grab spot
  (Transformation|AttachComponentToComponent (Variables|Default|GetStaticMesh1) (Variables|Default|GetGrabSpot) "None" "KeepWorld" "KeepWorld" "KeepWorld" true)
  ;;[0.1229 1 0.2293] Finally - attaching grab spot to controller
  (Transformation|AttachComponentToComponent (Variables|Default|GetGrabSpot) TargetComponent "None" "KeepWorld" "KeepWorld" "KeepWorld" false))

(fn OnReleaseDetachActor
  (params (Detaching%20Component :type Primitive%20Component%20Object%20Reference))
  (Transformation|DetachFromComponent (Variables|Default|GetGrabSpot) "KeepRelative" "KeepRelative" "KeepRelative" true))