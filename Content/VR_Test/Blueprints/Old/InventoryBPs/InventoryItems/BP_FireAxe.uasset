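; BP_FireAxe is a grabbable VR inventory item that damages BP_BreakableDoor actors when its blade hits them.
; A BladeCollision overlap applies durability damage and prints a debug message, with a DoOnce limiting it to one hit until the blade leaves that door.
; When grabbed by anything other than an inventory slot, it enables query and physics collision on the blade and mesh and makes the blade block WorldStatic.
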(event OnGrabbed(GrabComponent)
  (Utilities|Casting|CastToBP_InventorySlot (Components|GetOwner (Variables|/Game/VRTemplate/Blueprints/GrabComponent.GrabComponent_C|GetMotionControllerRef (Variables|Default|GetGrabComponent)))
    (:CastFailed
      (Collision|SetCollisionEnabled (Variables|Default|GetBlade) "QueryAndPhysics")
      (Collision|SetCollisionEnabled (Variables|Default|GetObjectMesh) "QueryAndPhysics")
      (Collision|SetCollisionResponsetoChannel (Variables|Default|GetBlade) "ECC_WorldStatic" "ECR_Block"))))

(event OnComponentBeginOverlap(BladeCollision)
  (params (OverlappedComponent :type Primitive%20Component%20Object%20Reference) (OtherActor :type Actor%20Object%20Reference) (OtherComp :type Primitive%20Component%20Object%20Reference) (OtherBodyIndex :type Integer) (bFromSweep :type Boolean) (SweepResult :type Hit%20Result%20Structure%20%28by%20ref%29))
  (Utilities|FlowControl|DoOnce false :!label _label
    (:Completed
      (bind _asbp_breakable_door (Utilities|Casting|CastToBP_BreakableDoor OtherActor)
        (:then
          (Variables|Default|SetCollidedDoor _asbp_breakable_door)
          (Default|TakeDurabilityDamage _asbp_breakable_door (Variables|Default|GetDamage))
          (Development|PrintString "Damage done" true true "(R=1.000000,G=0.118267,B=0.871186,A=1.000000)" 6.0))
        (:CastFailed
          (goto _label Reset))))))

(event OnComponentEndOverlap(BladeCollision)
  (params (OverlappedComponent :type Primitive%20Component%20Object%20Reference) (OtherActor :type Actor%20Object%20Reference) (OtherComp :type Primitive%20Component%20Object%20Reference) (OtherBodyIndex :type Integer))
  (if (== OtherActor (Variables|Default|GetCollidedDoor))
    (Utilities|FlowControl|DoOnce false) ; enters at Reset
  ))

(event EventBeginPlay
  (|CallParentFunction) ; This node is disabled and will not be called.\nDrag off pins to build functionality.
)

(event Collision|EventActorBeginOverlap
  (params (OtherActor :type Actor%20Object%20Reference))
  (|CallParentFunction OtherActor) ; This node is disabled and will not be called.\nDrag off pins to build functionality.
)

(event EventTick
  (params (DeltaSeconds :type Float%20%28single-precision%29))
  (|CallParentFunction DeltaSeconds) ; This node is disabled and will not be called.\nDrag off pins to build functionality.
)

(fn ConstructionScript
  (|CallParentFunction))