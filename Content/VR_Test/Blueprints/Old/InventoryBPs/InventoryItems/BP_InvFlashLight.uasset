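; VR inventory flashlight item that the player switches on and off with the trigger.
; A trigger press passes through a DoOnce into a FlipFlop that alternates the SpotLight between lit and zero intensity.
; Releasing the trigger resets the DoOnce, so each press toggles only once.
; BeginPlay, Tick and overlap events only forward to the parent class.
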(event EventBeginPlay
  (|CallParentFunction))

(event Collision|EventActorBeginOverlap
  (params (OtherActor :type Actor%20Object%20Reference))
  (|CallParentFunction OtherActor))

(event EventTick
  (params (DeltaSeconds :type Float%20%28single-precision%29))
  (|CallParentFunction DeltaSeconds))

(event EventTriggerPressed
  (bind _spotlight (Variables|Default|GetSpotLight))
  (Utilities|FlowControl|DoOnce false
    (:Completed
      (Utilities|FlowControl|FlipFlop
        (:A
          (Rendering|Components|Light|SetIntensity _spotlight 7e+03))
        (:B
          (Rendering|Components|Light|SetIntensity _spotlight 0.0))))))

(event EventTriggerReleased
  (bind _spotlight (Variables|Default|GetSpotLight))
  (Utilities|FlowControl|DoOnce false) ; enters at Reset
)

(fn ConstructionScript)