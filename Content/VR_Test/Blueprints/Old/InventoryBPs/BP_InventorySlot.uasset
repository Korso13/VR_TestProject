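; BP_InventorySlot is an inventory slot actor that holds an item overlapping its sphere, apparently for VR.
; Sphere overlaps track the hovered BP_InventoryItemClass and register the slot on that item, clearing both references when that item leaves.
; Put calls TryGrab on the item's GrabComponent with a MotionController, then moves the item to the slot and sets its mesh collision to query-only.
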(event OnComponentBeginOverlap(SlotSphere)
  (params (OverlappedComponent :type Primitive%20Component%20Object%20Reference) (OtherActor :type Actor%20Object%20Reference) (OtherComp :type Primitive%20Component%20Object%20Reference) (OtherBodyIndex :type Integer) (bFromSweep :type Boolean) (SweepResult :type Hit%20Result%20Structure%20%28by%20ref%29))
  ;[1 0.9511 0.295] Item hovered over the inventory slot
  (bind _asbp_inventory_item_class (Utilities|Casting|CastToBP_InventoryItemClass OtherActor)
    (:then
      (bind _output_get (Variables|Default|SetHeldInvItem _asbp_inventory_item_class))
      ;;[0.3895 0.3336 1] Register this inventory slot
      (Variables|/Game/VR_Test/Blueprints/Old/InventoryBPs/BP_InventoryItemClass.BP_InventoryItemClass_C|SetHoveredInventorySlotRef _output_get self))
    (:CastFailed
      (Development|PrintString "Cast to inv item failed" true true "(R=0.692708,G=0.050510,B=0.050510,A=1.000000)"))))

(event OnComponentEndOverlap(SlotSphere)
  (params (OverlappedComponent :type Primitive%20Component%20Object%20Reference) (OtherActor :type Actor%20Object%20Reference) (OtherComp :type Primitive%20Component%20Object%20Reference) (OtherBodyIndex :type Integer))
  ;[0.8185 0 1] Item removed from slot or hover-over is finished
  (bind _asbp_inventory_item_class (Utilities|Casting|CastToBP_InventoryItemClass OtherActor))
  ;;[1 0.2176 0.2574] If it's held\hovered over item...
  (if (== _asbp_inventory_item_class (Variables|Default|GetHeldInvItem))
    ;;[0.2758 1 0.5132] Reset variables to Null
    (Variables|/Game/VR_Test/Blueprints/Old/InventoryBPs/BP_InventoryItemClass.BP_InventoryItemClass_C|SetHoveredInventorySlotRef (Variables|Default|GetHeldInvItem) 0)
    (Variables|Default|SetHeldInvItem 0)))

(event Custom|Put
  (bind _heldinvitem (Variables|Default|GetHeldInvItem)
    (:then
      (bind _isheld (Default|TryGrab (Variables|/Game/VR_Test/Blueprints/BP_VRInteractionBase.BP_VRInteractionBase_C|GetGrabComponent _heldinvitem) (Variables|Default|GetMotionController)))
      (if _isheld
        (Transformation|SetActorLocation (Variables|Default|GetHeldInvItem) (Transformation|GetActorLocation) false false)
        (Collision|SetCollisionEnabled (Variables|/Game/VR_Test/Blueprints/BP_VRInteractionBase.BP_VRInteractionBase_C|GetObjectMesh (Variables|Default|GetHeldInvItem)) "QueryOnly")
        (else
          (Development|PrintString "Failed to hold item" true true "(R=1.000000,G=0.047235,B=0.000000,A=1.000000)"))))
    (:else
      (Development|PrintString "No item held" true true "(R=0.619792,G=0.189623,B=0.077781,A=1.000000)"))))

(event EventBeginPlay)

(event Collision|EventActorBeginOverlap
  (params (OtherActor :type Actor%20Object%20Reference)))

(event EventTick
  (params (DeltaSeconds :type Float%20%28single-precision%29)))

(fn ConstructionScript)