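; Short-lived physics debris actor that takes on a random mesh and removes itself after a set time, built on a parent that supplies GrabMesh.
; On BeginPlay it assigns the mesh and debris material, enables blocking collision and physics simulation, then destroys itself once the persistence delay ends.
; The random index only yields the first two of the three wired meshes, so the third never appears.
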(event EventBeginPlay
  (bind _grabmesh (Variables|Default|GetGrabMesh))
  (Components|StaticMesh|SetStaticMesh _grabmesh (Utilities|Select :Index (Math|Random|RandomInteger 2) :Option%200 "/Game/VR_Test/Meshes/SM_Debris01.SM_Debris01" :Option%201 "/Game/VR_Test/Meshes/SM_Debris02.SM_Debris02" :Option%202 "/Game/VR_Test/Meshes/SM_Debris03.SM_Debris03"))
  (Rendering|Material|SetMaterial _grabmesh 0 (Variables|Default|GetDebrisMaterial))
  (Collision|SetCollisionEnabled _grabmesh "QueryAndPhysics")
  (Collision|SetCollisionResponsetoAllChannels _grabmesh "ECR_Block")
  (Physics|SetSimulatePhysics _grabmesh true)
  (Utilities|FlowControl|Delay (Variables|Default|GetDebrisPersistanceTime))
  (Actor|DestroyActor))

(event Collision|EventActorBeginOverlap
  (params (OtherActor :type Actor%20Object%20Reference)))

(event EventTick
  (params (DeltaSeconds :type Float%20%28single-precision%29)))

(fn ConstructionScript
  (|CallParentFunction))