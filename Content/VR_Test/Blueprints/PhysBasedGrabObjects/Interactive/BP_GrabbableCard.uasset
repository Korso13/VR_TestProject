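; BP_GrabbableCard is a physics-based grabbable card for VR that attaches to the interacting component at the point of contact.
; When its GrabComponent is not using the standard attachment method, BeginPlay binds custom handlers to grab and drop.
; Grab disables physics, moves GrabSpot to the closest collision point, then chains GrabComponent to GrabSpot and GrabSpot to the interacting component.
; Drop re-enables physics and detaches GrabComponent.
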(event Custom|Grab
  (params (Interacting%20Component :type Primitive%20Component%20Object%20Reference))
  (Physics|SetSimulatePhysics (Variables|Default|GetGrabComponent) false)
  ;[0.191 0.2518 1] Moving grab spot to closest point on item's collision
  (Transformation|SetWorldLocation (Variables|Default|GetGrabSpot) (.OutPointOnBody (Collision|GetClosestPointonCollision (Variables|Default|GetGrabComponent) (Transformation|GetWorldLocation Interacting%20Component) "None")) false false)
  ;[0.191 0.2518 1] Forcing the main mesh to follow grab spot
  (Transformation|AttachComponentToComponent (Variables|Default|GetGrabComponent) (Variables|Default|GetGrabSpot) "None" "KeepWorld" "KeepWorld" "KeepWorld" true)
  ;[0.1229 1 0.2293] Finally - attaching grab spot to controller
  (Transformation|AttachComponentToComponent (Variables|Default|GetGrabSpot) Interacting%20Component "None" "KeepWorld" "KeepWorld" "KeepWorld" false))

(event Custom|Drop
  (bind _grabcomponent (Variables|Default|GetGrabComponent))
  (Physics|SetSimulatePhysics _grabcomponent true)
  (Transformation|DetachFromComponent _grabcomponent "KeepWorld" "KeepWorld" "KeepWorld" true))

(event EventBeginPlay
  (bind _grabcomponent (Variables|Default|GetGrabComponent))
  (if (not (Variables|/Game/VR_Test/Components/BPC_GrabComponent.BPC_GrabComponent_C|GetbUseStandardAttachmentMethod _grabcomponent))
    (EventDispatchers|BindEventtoOnGrab _grabcomponent (EventDispatchers|CreateEvent :!event Custom|Grab))
    (EventDispatchers|BindEventtoOnDrop _grabcomponent (EventDispatchers|CreateEvent :!event Custom|Drop))))

(event Collision|EventActorBeginOverlap
  (params (OtherActor :type Actor%20Object%20Reference)))

(event EventTick
  (params (DeltaSeconds :type Float%20%28single-precision%29)))

(fn ConstructionScript
  (|CallParentFunction))